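; Trigger-volume actor that plays the boat wood-creak soundscape palette while the player is inside its box.
; On player overlap it spawns SPalette_Boat_Wood_Creaks, stores the active palette and plays it.
; When the player leaves, it stops that palette, with an IsInside flag guarding against duplicate starts and stops.
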(event OnComponentBeginOverlap(Box)
  (params (OverlappedComponent :type Primitive%20Component%20Object%20Reference) (OtherActor :type Actor%20Object%20Reference) (OtherComp :type Primitive%20Component%20Object%20Reference) (OtherBodyIndex :type Integer) (bFromSweep :type Boolean) (SweepResult :type Hit%20Result%20Structure%20%28by%20ref%29))
  (if (== OtherActor (Game|GetPlayerCharacter 0))
    (if (not (Variables|Default|GetisInside))
      (bind _soundscapepaletteagentsout (Class|SoundscapeBPFunctionLibrary|SpawnSoundscapePalette "/Game/Audio/Sound/Environnement/Ship/Boat_Wood_Creaks/SPalette_Boat_Wood_Creaks.SPalette_Boat_Wood_Creaks"))
      (bind _output_get (Variables|Default|SetActivePalette _soundscapepaletteagentsout))
      (Class|ActiveSoundscapePalette|Play _output_get)
      (Variables|Default|SetisInside true))))

(event OnComponentEndOverlap(Box)
  (params (OverlappedComponent :type Primitive%20Component%20Object%20Reference) (OtherActor :type Actor%20Object%20Reference) (OtherComp :type Primitive%20Component%20Object%20Reference) (OtherBodyIndex :type Integer))
  (if (== OtherActor (Game|GetPlayerCharacter 0))
    (if (Variables|Default|GetisInside)
      (bind _activepalette (Variables|Default|GetActivePalette)
        (:then
          (Class|ActiveSoundscapePalette|Stop _activepalette)
          (Variables|Default|SetisInside false))
        (:else)))))

(event EventBeginPlay)

(event Collision|EventActorBeginOverlap
  (params (OtherActor :type Actor%20Object%20Reference)))

(event EventTick
  (params (DeltaSeconds :type Float%20%28single-precision%29)))

(fn ConstructionScript)