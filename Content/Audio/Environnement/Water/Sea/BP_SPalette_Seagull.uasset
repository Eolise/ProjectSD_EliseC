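; Sea-environment audio actor that plays the seagull ambience through a Soundscape palette.
; On BeginPlay it spawns the SPalette_Seagull palette, stores the agent as ActivePalette and plays it, so the ambience starts unconditionally.
; Box overlap events are empty; the player-only enter/exit logic that would start and stop the palette using an IsInside flag is disconnected and never runs.
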(event OnComponentBeginOverlap(Box)
  (params (OverlappedComponent :type Primitive%20Component%20Object%20Reference) (OtherActor :type Actor%20Object%20Reference) (OtherComp :type Primitive%20Component%20Object%20Reference) (OtherBodyIndex :type Integer) (bFromSweep :type Boolean) (SweepResult :type Hit%20Result%20Structure%20%28by%20ref%29)))

(event OnComponentEndOverlap(Box)
  (params (OverlappedComponent :type Primitive%20Component%20Object%20Reference) (OtherActor :type Actor%20Object%20Reference) (OtherComp :type Primitive%20Component%20Object%20Reference) (OtherBodyIndex :type Integer)))

(event EventBeginPlay
  (bind _soundscapepaletteagentsout (Class|SoundscapeBPFunctionLibrary|SpawnSoundscapePalette "/Game/Audio/Environnement/Water/Sea/SPalette_Seagull.SPalette_Seagull"))
  (bind _output_get (Variables|Default|SetActivePalette _soundscapepaletteagentsout))
  (Class|ActiveSoundscapePalette|Play _output_get))

(event Collision|EventActorBeginOverlap
  (params (OtherActor :type Actor%20Object%20Reference)))

(event EventTick
  (params (DeltaSeconds :type Float%20%28single-precision%29)))

(fn ConstructionScript)